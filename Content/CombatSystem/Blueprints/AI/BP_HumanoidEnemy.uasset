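; BP_HumanoidEnemy is a humanoid AI enemy in the combat system that adds a health bar to its parent class.
; On BeginPlay it creates a WB_HealthBar bound to its own StatsComponent rather than the player's and assigns it to the HealthBar widget component.
; The OnTargeted override calls the parent, then sets the bar's visibility to match the targeted state.
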(event `self.ReceiveBeginPlay`
  (`parent.ReceiveBeginPlay`)
  (bind _returnvalue (`|CreateWidget` "/Game/CombatSystem/UI/WB_HealthBar.WB_HealthBar_C" (`GameplayStatics.GetPlayerController` 0) (`self.StatsComponent`) false))
  (`WidgetComponent.SetWidget` (`self.HealthBar`) _returnvalue))

(event `/Game/CombatSystem/Blueprints/Interfaces/TargetingBPI.OnTargeted`
  (params (`bIsTargeted?` :type Boolean))
  (`parent.OnTargeted` `bIsTargeted?`)
  (`SceneComponent.SetVisibility` (`self.HealthBar`) `bIsTargeted?` false))

(fn `UserConstructionScript`
  (`parent.UserConstructionScript`))