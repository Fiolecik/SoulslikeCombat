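; Combat actor component that detects hits along a mesh, likely a weapon, during activated collision windows.
; While enabled, each Tick runs a multi-sphere object trace between two sockets on the assigned mesh, skipping ignored actors.
; CanHitActor rejects already-hit actors, ignored classes and ignored gameplay tags; accepted hits are recorded and broadcast through OnHit.
; Activation clears the hit list, so each actor registers only once per window.
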(event `SetCollisionMesh`
  (params (MeshComponent :type "PrimitiveComponent Object Reference"))
  ;[1 0 0.02745] Set Collision Mesh component
  (set `self.CollisionMeshComponent` MeshComponent))

(event `self.ReceiveTick`
  (params (DeltaSeconds :type "Float (single-precision)"))
  (if (`self.bIsCollisionEnabled?`)
    (`self.CollisionTrace`)))

(event `ActivateCollision`
  ;[1 0 0.02745] Activate Collision
  (`self.ClearHitActors`)
  (set `self.bIsCollisionEnabled?` true))

(event `CollisionTrace`
  (bind _collisionmeshcomponent (`self.CollisionMeshComponent`))
  ;[1 0 0.02745] CollisionTrace
  (bind _outhits (`KismetSystemLibrary.SphereTraceMultiForObjects` (`SceneComponent.GetSocketLocation` _collisionmeshcomponent (`self.StartSocketName`)) (`SceneComponent.GetSocketLocation` _collisionmeshcomponent (`self.EndSocketName`)) (`self.TraceRadius`) (`self.CollisionObjectTypes`) false (`self.ActorsIgnore`) (`self.Draw Debug Type`)))
  (for _array_element _outhits
    (bind _output_get (set `self.LastHit` _array_element))
    (bind (_bblockinghit _binitialoverlap _time _distance _location _impactpoint _normal _impactnormal _physmat _hitactor) (`GameplayStatics.BreakHitResult` _output_get))
    (if (`self.CanHitActor?` _hitactor)
      (bind _output_get_2 (set `self.Hit Actor` _hitactor))
      (`KismetArrayLibrary.Array_Add` (`self.AlreadyHitActors`) _output_get_2)
      (`self.OnHit` (`self.LastHit`)))))

(event `DeactivateCollision`
  ;[1 0 0.02745] Deactivate Collision
  (set `self.bIsCollisionEnabled?` false))

(event `ClearHitActors`
  ;[1 0 0.02745] Clear Hit Actors
  (`KismetArrayLibrary.Array_Clear` (`self.AlreadyHitActors`)))

(fn `AddActorToIgnore`
  (params (InActor :type "Actor Object Reference (by ref)"))
  (`KismetArrayLibrary.Array_AddUnique` (`self.ActorsIgnore`) InActor))

(fn `CanHitActor?`
  (params (InActor :type "Actor Object Reference (by ref)"))
  (returns (ReturnValue :type Boolean))
  (bind _returnvalue (message `/Game/CombatSystem/Blueprints/Interfaces/GameplayTagBlueprintInterface.GetOwnedGameplayTags` InActor))
  (return (and (not (`KismetArrayLibrary.Array_Contains` (`self.AlreadyHitActors`) InActor)) (not (`KismetArrayLibrary.Array_Contains` (`self.Actors to Ignore`) (`GameplayStatics.GetObjectClass` (`local.InActor`)))) (not (`BlueprintGameplayTagLibrary.HasAnyTags` _returnvalue (`self.GameplayTagsToIgnore`) true)))))

(fn `GetActorsToIgnore`
  (returns (ReturnValue :type "Array of Actor Object Reference"))
  (return (`self.ActorsIgnore`)))

(fn `GetAlreadyHitActors`
  (returns (ReturnValue :type "Array of Actor Object Reference"))
  (return (`self.AlreadyHitActors`)))

(fn `GetCollisionMeshComponent`
  (returns (ReturnValue :type "PrimitiveComponent Object Reference"))
  (return (`self.CollisionMeshComponent`)))

(fn `GetLastHit`
  (returns (ReturnValue :type "HitResult Structure"))
  (return (`self.LastHit`)))

(fn `IsCollisionEnabled?`
  (returns (ReturnValue :type Boolean))
  (return (`self.bIsCollisionEnabled?`)))

(fn `RemoveActorToIgnore`
  (params (InActorToRemove :type "Actor Object Reference (by ref)"))
  (`KismetArrayLibrary.Array_RemoveItem` (`self.ActorsIgnore`) InActorToRemove))