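; Test dummy character for the combat system that can be targeted and receive damage while it is not in the Dead state.
; On BeginPlay it initializes its stats, spawns and equips its starting equipment, and prints a current stat value for debugging.
; Targeting events toggle its lock-on widget, and both the damage and targetability checks query the state manager component.
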(event `self.ReceiveBeginPlay`
  (`/Game/CombatSystem/Blueprints/Components/StatsComponent.InitializeStats` (`self.StatsComponent`))
  (for _array_element (`self.StartingEquipment`)
    (bind _returnvalue (`|SpawnActorFromClass` _array_element (`self.GetTransform`) "Undefined" "OverrideRootScale" self self))
    (`/Game/CombatSystem/Blueprints/Actors/BP_BaseEquippable.OnEquipped` _returnvalue))
  (`KismetSystemLibrary.PrintString` (`KismetStringLibrary.Conv_DoubleToString` (`/Game/CombatSystem/Blueprints/Components/StatsComponent.GetCurrentStatValue` (`self.StatsComponent`) "NewEnumerator3"))))

(event `/Game/CombatSystem/Blueprints/Interfaces/TargetingBPI.OnTargeted`
  (params (`bIsTargeted?` :type Boolean))
  (`SceneComponent.SetVisibility` (`self.LockOnWidget`) `bIsTargeted?` false))

(fn `CanBeTargeted?`
  (returns (ReturnValue :type Boolean))
  (return (not (`/Game/CombatSystem/Blueprints/Components/StateManagerComponent.IsCurrentStateEqualToAny?` (`self.StateManagerComponent`) (struct :`GameplayTags` (struct :`(TagName` "Character.State.Dead")))))))

(fn `CanRecieveDamage`
  (returns (ReturnValue :type Boolean))
  (return (not (`/Game/CombatSystem/Blueprints/Components/StateManagerComponent.IsCurrentStateEqualToAny?` (`self.StateManagerComponent`) (struct :`GameplayTags` (struct :`(TagName` "Character.State.Dead")))))))

(fn `UserConstructionScript`
  (`parent.UserConstructionScript`))